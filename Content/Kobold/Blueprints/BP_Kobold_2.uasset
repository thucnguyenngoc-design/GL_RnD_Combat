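; BP_Kobold_2 is a Kobold Blueprint with a modular body of decor, armor and sword meshes.
; Its construction script sets the main Mesh as master pose component for three item meshes and the armor, so they share its animation.
; Exposed-style visibility variables then toggle the sword, armor and two of the decor items, allowing different looks per instance.
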(fn ConstructionScript
  (Class|SkinnedMeshComponent|SetMasterPoseComponent (Variables|Default|GetSKM_Item1) (Variables|Character|GetMesh) true)
  (Utilities|FlowControl|Sequence
    (:then_0
      (Rendering|SetVisibility (Variables|Default|GetSKM_Item3) (Variables|Default|GetDecor2_Visibility) false))
    (:then_1
      (Rendering|SetVisibility (Variables|Default|GetSM_Sword) (Variables|Default|GetWeapon_Visibility) false))
    (:then_3
      (Rendering|SetVisibility (Variables|Default|GetSKM_Armor) (Variables|Default|GetArmor_Visibility) false))
    (:then_7
      (Rendering|SetVisibility (Variables|Default|GetSKM_Item1) (Variables|Default|GetDecor1_Visibility) false))))