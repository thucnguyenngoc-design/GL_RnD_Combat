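; BP_VideoPlayer is a prototype Blueprint that switches a media player between three videos, named for Souls-like, fast-paced and survival themes.
; Each theme has its own event, which stores a fixed index in PlayMedia and passes it to PlayVideoMedia.
; That function opens the matching VideoArray entry as the source on Media, with no explicit play call or bounds check.
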(event EventSurvivalVideo
  (bind _output_get (Variables|Default|SetPlayMedia 2))
  (CallFunction|PlayVideoMedia _output_get))

(event EventSoulLikeVideo
  (bind _output_get (Variables|Default|SetPlayMedia 0))
  (CallFunction|PlayVideoMedia _output_get))

(event EventFastPacedVideo
  (bind _output_get (Variables|Default|SetPlayMedia 1))
  (CallFunction|PlayVideoMedia _output_get))

(fn ConstructionScript)

(fn PlayVideoMedia
  (params (VideoIndex :type Integer))
  (Media|MediaPlayer|OpenSource (Variables|Default|GetMedia) (Utilities|Array|Get(acopy) (Variables|Default|GetVideoArray) VideoIndex)))