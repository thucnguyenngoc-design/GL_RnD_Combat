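; BP_Chain_FastPaced is the Fast Paced option on a config board, selected by overlapping its collision box.
; Selection highlights its mesh and text, locks it against toggling off, and has BP_VideoPlayer show the matching video.
; It then messages the Survival, Soul Like and Flow Combat options, found by class, while its own FastPacedControl event clears its selection.
; Each overlap also switches the touching component to physics-only collision.
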(event OnComponentBeginOverlap(BoxCollision)
  (params (OverlappedComponent :type Primitive%20Component%20Object%20Reference) (OtherActor :type Actor%20Object%20Reference) (OtherComp :type Primitive%20Component%20Object%20Reference) (OtherBodyIndex :type Integer) (bFromSweep :type Boolean) (SweepResult :type Hit%20Result%20Structure%20%28by%20ref%29))
  (Utilities|FlowControl|DoOnce false :!label _label
    (:Completed
      (Utilities|FlowControl|Sequence
        (:then_0
          (if (not (Variables|Default|GetisActivate))
            (Variables|Default|SetisActivate true)
            (Rendering|Material|SetOverlayMaterial (Variables|Default|Getcb) "/Game/Prototype/Material/M_Selection.M_Selection" :!class /Script/Engine.MeshComponent)
            (Rendering|Components|TextRender|SetTextRenderColor (Variables|Default|GetTextRender) (Math|Conversions|ToColor(LinearColor) (Variables|Default|GetGreenColor)))
            (Variables|Default|SetPlayVideo true)
            (bind _returnvalue (Actor|GetActorOfClass "/Game/Prototype/Blueprints/BP_VideoPlayer.BP_VideoPlayer_C"))
            (Class|BPIChangeVideo|FastPacedVideo(Message) _returnvalue)
            (Variables|Default|SetLockOption true)
            (Utilities|FlowControl|Sequence
              (:then_0
                (bind _returnvalue_2 (Actor|GetActorOfClass "/Game/Prototype/Blueprints/BP_ConfigBoard/BP_Chain_Survival.BP_Chain_Survival_C"))
                (Class|BPIBoardManager|SurvivalControl(Message) _returnvalue_2))
              (:then_1
                (bind _returnvalue_3 (Actor|GetActorOfClass "/Game/Prototype/Blueprints/BP_ConfigBoard/BP_Chain_Soul_Like.BP_Chain_Soul_Like_C"))
                (Class|BPIBoardManager|SoulLikeControl(Message) _returnvalue_3))
              (:then_2
                (bind _returnvalue_4 (Actor|GetActorOfClass "/Game/Prototype/Blueprints/BP_ConfigBoard/BP_Chain_FlowCombat.BP_Chain_FlowCombat_C"))
                (Class|BPIBoardManager|FlowCombatControl(Message) _returnvalue_4)))
            (elif (not (Variables|Default|GetLockOption))
              (Variables|Default|SetisActivate false)
              (Rendering|Material|SetOverlayMaterial (Variables|Default|Getcb) 0 :!class /Script/Engine.MeshComponent)
              (Rendering|Components|TextRender|SetTextRenderColor (Variables|Default|GetTextRender) (Math|Conversions|ToColor(LinearColor) (Variables|Default|GetWhiteColor)))
              (Variables|Default|SetPlayVideo false))))
        (:then_1
          (Collision|SetCollisionEnabled OtherComp "PhysicsOnly")
          (goto _label Reset))))))

(event EventFastPacedControl
  (Variables|Default|SetLockOption false)
  (Variables|Default|SetisActivate false)
  (Rendering|Material|SetOverlayMaterial (Variables|Default|Getcb) 0 :!class /Script/Engine.MeshComponent)
  (Rendering|Components|TextRender|SetTextRenderColor (Variables|Default|GetTextRender) (Math|Conversions|ToColor(LinearColor) (Variables|Default|GetWhiteColor))))

(fn ConstructionScript)