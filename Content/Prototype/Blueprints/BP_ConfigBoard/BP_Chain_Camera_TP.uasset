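; BP_Chain_Camera_TP is an overlap-triggered toggle on the config board for the third-person camera option, highlighted blue and active at start.
; When activated by an overlap, it locks itself and messages BP_Chain_Camera_TopDown, forming a mutually exclusive pair.
; TPCamControl unlocks and deactivates it, clearing the overlay and whitening the text.
; Each hit sets the overlapping component to physics-only collision, with a DoOnce guarding re-entry.
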(event OnComponentBeginOverlap(BoxCollision)
  (params (OverlappedComponent :type Primitive%20Component%20Object%20Reference) (OtherActor :type Actor%20Object%20Reference) (OtherComp :type Primitive%20Component%20Object%20Reference) (OtherBodyIndex :type Integer) (bFromSweep :type Boolean) (SweepResult :type Hit%20Result%20Structure%20%28by%20ref%29))
  (Utilities|FlowControl|DoOnce false :!label _label
    (:Completed
      (Utilities|FlowControl|Sequence
        (:then_0
          (if (not (Variables|Default|GetisActivate))
            (Variables|Default|SetisActivate true)
            (Rendering|Material|SetOverlayMaterial (Variables|Default|Getcb) "/Game/Prototype/Material/M_Selection_Blue.M_Selection_Blue" :!class /Script/Engine.MeshComponent)
            (Rendering|Components|TextRender|SetTextRenderColor (Variables|Default|GetTextRender) (Math|Conversions|ToColor(LinearColor) (Variables|Default|GetBlueColor)))
            (Variables|Default|SetLockOption true)
            (bind _returnvalue (Actor|GetActorOfClass "/Game/Prototype/Blueprints/BP_ConfigBoard/BP_Chain_Camera_TopDown.BP_Chain_Camera_TopDown_C"))
            (Class|BPIBoardManager|TopDownCamControl(Message) _returnvalue)
            (elif (not (Variables|Default|GetLockOption))
              (Variables|Default|SetisActivate false)
              (Rendering|Material|SetOverlayMaterial (Variables|Default|Getcb) 0 :!class /Script/Engine.MeshComponent)
              (Rendering|Components|TextRender|SetTextRenderColor (Variables|Default|GetTextRender) (Math|Conversions|ToColor(LinearColor) (Variables|Default|GetWhiteColor))))))
        (:then_1
          (Collision|SetCollisionEnabled OtherComp "PhysicsOnly")
          (goto _label Reset))))))

(event EventBeginPlay
  (Variables|Default|SetisActivate true)
  (Rendering|Material|SetOverlayMaterial (Variables|Default|Getcb) "/Game/Prototype/Material/M_Selection_Blue.M_Selection_Blue" :!class /Script/Engine.MeshComponent)
  (Rendering|Components|TextRender|SetTextRenderColor (Variables|Default|GetTextRender) (Math|Conversions|ToColor(LinearColor) (Variables|Default|GetBlueColor))))

(event EventTPCamControl
  (Variables|Default|SetLockOption false)
  (Variables|Default|SetisActivate false)
  (Rendering|Material|SetOverlayMaterial (Variables|Default|Getcb) 0 :!class /Script/Engine.MeshComponent)
  (Rendering|Components|TextRender|SetTextRenderColor (Variables|Default|GetTextRender) (Math|Conversions|ToColor(LinearColor) (Variables|Default|GetWhiteColor))))

(fn ConstructionScript)